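; BP_Background is an actor that plays a background video through a Media Player.
; On BeginPlay it opens the Background media source, starts playback and binds a handler to the end-reached event.
; Each time the media ends, the handler flips a Rate boolean, sets the playback rate to either zero or reverse accordingly, then immediately calls Play again.
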(event `self.ReceiveBeginPlay`
  (`MediaPlayer.OpenSource` (`self.MediaPlayer`) "/Game/Movies/Background.Background")
  (`MediaPlayer.Play` (`self.MediaPlayer`))
  (add `MediaPlayer.OnEndReached` (`self.MediaPlayer`) (delegate `OnEndReached`)))

(event `OnEndReached`
  (set `self.Rate` (not (`self.Rate`)))
  (if (`self.Rate`)
    (`MediaPlayer.SetRate` (`self.MediaPlayer`) 0.0)
    (else
      (`MediaPlayer.SetRate` (`self.MediaPlayer`) -1.0)))
  (`MediaPlayer.Play` (`self.MediaPlayer`)))

(fn `UserConstructionScript`)