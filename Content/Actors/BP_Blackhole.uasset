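; BP_Blackhole is a black hole actor with a sphere that travels along a spline and a radial force that attracts physics objects.
; The construction script gives the RadialForce component a very large radius and a strong negative strength, producing the inward pull.
; BeginPlay caches the spline length, and Tick advances the sphere by distance at MoveSpeed, snapping back to the start past the end.
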(event `self.ReceiveBeginPlay`
  (set `self.TotalSplineLength` (`SplineComponent.GetSplineLength` (`self.Spline`))))

(event `self.ReceiveTick`
  (params (DeltaSeconds :type "Float (single-precision)"))
  (set `self.CurrentDistance` (+ (* DeltaSeconds (`self.MoveSpeed`)) (`self.CurrentDistance`)))
  (if (> (`self.CurrentDistance`) (`self.TotalSplineLength`))
    (set `self.CurrentDistance` 0.0))
  (`SceneComponent.K2_SetWorldLocation` (`self.Sphere`) (`SplineComponent.GetLocationAtDistanceAlongSpline` (`self.Spline`) (`self.CurrentDistance`) "World") false false))

(fn `UserConstructionScript`
  (set `RadialForceComponent.Radius` 10000.0 (`self.RadialForce`))
  (set `RadialForceComponent.ForceStrength` -10000000.0 (`self.RadialForce`)))